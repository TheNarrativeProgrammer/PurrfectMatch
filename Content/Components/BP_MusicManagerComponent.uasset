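; Music manager component that drives the game's main soundtrack across the main menu, story menu and gameplay.
; On BeginPlay it reuses the track stored in BP_GameInstancePM, or creates MS_MainTrack as a 2D sound that persists across level transitions, stores it there and fades it in.
; Events switch music states through named trigger parameters on that single MetaSound, or stop playback entirely.
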(event `self.ReceiveBeginPlay`
  (bind _asbp_game_instance_pm (cast `/Game/Core/BP_GameInstancePM` (`GameplayStatics.GetGameInstance`)))
  (set `self.As BP Game Instance PM` _asbp_game_instance_pm)
  (bind _newparam (`/Game/Core/BP_GameInstancePM.GetMainTrack` (`self.As BP Game Instance PM`)))
  (`/Engine/EditorBlueprintResources/StandardMacros.IsValid` _newparam
    (:`Is Valid`
      (set `self.MainTrack` _newparam))
    (:`Is Not Valid`
      (bind _returnvalue (`GameplayStatics.CreateSound2D` "/Game/Music/MetaSounds/MS_MainTrack.MS_MainTrack" 1.0 1.0 0.0 null true false))
      (bind _output_get (set `self.MainTrack` _returnvalue))
      (`/Game/Core/BP_GameInstancePM.SetMainTrack` (`self.As BP Game Instance PM`) _output_get)
      (`self.InitializeMainTrack`))))

(event `InitializeMainTrack`
  (bind _maintrack (`self.MainTrack`))
  ; Initialize track when game begins
  (`/Engine/EditorBlueprintResources/StandardMacros.IsValid` _maintrack
    (:`Is Valid`
      (`AudioComponent.FadeIn` _maintrack 6.0 1.0 0.0 "Linear")
      (`AudioParameterControllerInterface.SetTriggerParameter` (`self.MainTrack`) "PlayMainMenu"))))

(event `StopMusic`
  ; Play Main menu music
  (`/Engine/EditorBlueprintResources/StandardMacros.IsValid` (`self.MainTrack`)
    (:`Is Valid`
      (`AudioComponent.Stop` (`self.MainTrack`)))))

(event `PlayMainMenuMusic`
  ; Play Main menu music
  (`/Engine/EditorBlueprintResources/StandardMacros.IsValid` (`self.MainTrack`)
    (:`Is Valid`
      (`AudioParameterControllerInterface.SetTriggerParameter` (`self.MainTrack`) "PlayMainMenu"))))

(event `PlayGamePlayMusic`
  ; Play Main menu music
  (`/Engine/EditorBlueprintResources/StandardMacros.IsValid` (`self.MainTrack`)
    (:`Is Valid`
      (`AudioParameterControllerInterface.SetTriggerParameter` (`self.MainTrack`) "PlayGamePlay"))))

(event `PlayStoryMenuMusic`
  ; Play Main menu music
  (`/Engine/EditorBlueprintResources/StandardMacros.IsValid` (`self.MainTrack`)
    (:`Is Valid`
      (`AudioParameterControllerInterface.SetTriggerParameter` (`self.MainTrack`) "PlayStoryMenu"))))