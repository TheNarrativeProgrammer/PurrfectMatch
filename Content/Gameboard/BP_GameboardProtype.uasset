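; Prototype gameboard actor that builds a flat grid of plane tiles in its construction script, with no gameplay logic.
; Nested loops over Height and Width add a blue-material static mesh per cell, store it in Planes and attach it to Scene.
; PlaneLocation offsets each cell index by GridOrigin and scales by TileSize at zero Z.
; GetIndex computes a row-major index, stored in IndexOfArray.
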(fn `GetIndex`
  (params (X :type Integer) (Y :type Integer))
  (returns (Index :type Integer))
  (return (+ X (* Y (`self.width`)))))

(fn `PlaneLocation`
  (params (XIndex :type Integer) (YIndex :type Integer))
  (returns (Location :type "Vector Structure"))
  (locals (PlaneLocation :type "Vector Structure" :default (0.0 0.0 0.0)))
  (bind (_planelocation_x _planelocation_y) (`KismetMathLibrary.BreakVector` (`local.PlaneLocation`)))
  (set `local.PlaneLocation` (`self.GridOrigin`))
  (return (`KismetMathLibrary.MakeVector` (* (+ XIndex _planelocation_x) (`self.TileSize`)) (* (+ _planelocation_y YIndex) (`self.TileSize`)))))

(fn `UserConstructionScript`
  (locals (XValue :type Integer) (YValue :type Integer))
  (for _index (range (+ (`self.Height`) 1))
    (set `local.YValue` _index)
    (for _index_2 (range (+ (`self.width`) 1))
      (set `local.XValue` _index_2)
      (bind _index_3 (`self.GetIndex` _index_2 _index))
      (set `self.IndexOfArray` _index_3)
      (bind _location (`self.PlaneLocation` (`local.XValue`) (`local.YValue`)))
      (bind _returnvalue (`AddComponent|NODE_AddStaticMeshComponent-0`))
      (bind _output_get (set `self.CurrentPlane` _returnvalue))
      (`SceneComponent.K2_SetWorldLocation` _output_get _location false false)
      (`StaticMeshComponent.SetStaticMesh` _output_get "/Engine/BasicShapes/Plane.Plane")
      (`PrimitiveComponent.SetMaterial` (`self.CurrentPlane`) 0 "/AnimationSharing/AnimSharingBlue.AnimSharingBlue")
      (`KismetArrayLibrary.Array_AddUnique` (`self.Planes`) (`self.CurrentPlane`))
      (`SceneComponent.K2_AttachToComponent` (`self.CurrentPlane`) (`self.Scene`) "None" "KeepRelative" "KeepRelative" "KeepRelative" true))))